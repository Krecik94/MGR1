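; Pressure button for Level1 that activates connected actors while anything overlaps it.
; The first overlapping actor instantly lowers the Button component, sets Pushed and calls ButtonActivate on each entry in ConnectedActors.
; When the last overlapping actor leaves, the component moves back, Pushed clears and each connected actor receives ButtonDeactivate.
; Overlap counts and the Pushed flag prevent repeat triggers when several actors share the button.
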(event Collision|EventActorBeginOverlap
  (params (OtherActor :type Actor%20Object%20Reference))
  (bind _connected_actors (Variables|Public|GetConnected%20Actors))
  (if (not (> (Utilities|Array|Length (Collision|GetOverlappingActors "/Script/Engine.Actor" :!class /Script/Engine.Actor)) 1))
    (if (not (Variables|Default|GetPushed))
      (Components|MoveComponentTo (Variables|Default|GetButton) "0, 0,-10.000000" "0, 0, 0" false false 0.0 false)
      (Variables|Default|SetPushed true)
      (for _array_element _connected_actors
        (Default|ButtonActivate _connected_actors)))))

(event Collision|EventActorEndOverlap
  (params (OtherActor :type Actor%20Object%20Reference))
  (bind _connected_actors (Variables|Public|GetConnected%20Actors))
  (if (not (> (Utilities|Array|Length (Collision|GetOverlappingActors "/Script/Engine.Actor" :!class /Script/Engine.Actor)) 0))
    (if (Variables|Default|GetPushed)
      (Components|MoveComponentTo (Variables|Default|GetButton) "0, 0, 0" "0, 0, 0" false false 0.0 false)
      (Variables|Default|SetPushed false)
      (for _array_element _connected_actors
        (Default|ButtonDeactivate _connected_actors)))))

(fn ConstructionScript)