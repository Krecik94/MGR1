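; Finish zone actor for Level1 that shows the win screen once two players are inside it at the same time.
; Overlap begin and end events raise or lower a PlayersInside count for Player actors only.
; The count drives two mesh indicators, turning Sphere green at one player and both Sphere and StaticMesh green at two, when it also creates and displays the Win_Screen widget.
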(event Collision|EventActorBeginOverlap
  (params (OtherActor :type Actor%20Object%20Reference))
  (Utilities|Casting|CastToPlayer OtherActor)
  (Variables|Default|SetPlayers_Inside (+ (Variables|Default|GetPlayers_Inside) 1))
  (switch int (Variables|Default|GetPlayers_Inside)
    (:0
      (Rendering|Material|SetMaterial (Variables|Default|GetSphere) 0 "/Game/Level1/Materials/Basic_Red.Basic_Red")
      (Rendering|Material|SetMaterial (Variables|Default|GetStaticMesh) 0 "/Game/Level1/Materials/Basic_Red.Basic_Red"))
    (:1
      (Rendering|Material|SetMaterial (Variables|Default|GetSphere) 0 "/Game/Level1/Materials/Basic_Green.Basic_Green")
      (Rendering|Material|SetMaterial (Variables|Default|GetStaticMesh) 0 "/Game/Level1/Materials/Basic_Red.Basic_Red"))
    (:2
      (Rendering|Material|SetMaterial (Variables|Default|GetSphere) 0 "/Game/Level1/Materials/Basic_Green.Basic_Green")
      (Rendering|Material|SetMaterial (Variables|Default|GetStaticMesh) 0 "/Game/Level1/Materials/Basic_Green.Basic_Green")
      (bind _returnvalue (UserInterface|CreateWidget "/Game/Level1/Win_Screen.Win_Screen_C"))
      (UserInterface|Viewport|AddtoViewport _returnvalue 0))))

(event Collision|EventActorEndOverlap
  (params (OtherActor :type Actor%20Object%20Reference))
  (Utilities|Casting|CastToPlayer OtherActor)
  (Variables|Default|SetPlayers_Inside (- (Variables|Default|GetPlayers_Inside) 1))
  (switch int (Variables|Default|GetPlayers_Inside)
    (:0
      (Rendering|Material|SetMaterial (Variables|Default|GetSphere) 0 "/Game/Level1/Materials/Basic_Red.Basic_Red")
      (Rendering|Material|SetMaterial (Variables|Default|GetStaticMesh) 0 "/Game/Level1/Materials/Basic_Red.Basic_Red"))
    (:1
      (Rendering|Material|SetMaterial (Variables|Default|GetSphere) 0 "/Game/Level1/Materials/Basic_Green.Basic_Green")
      (Rendering|Material|SetMaterial (Variables|Default|GetStaticMesh) 0 "/Game/Level1/Materials/Basic_Red.Basic_Red"))
    (:2
      (Rendering|Material|SetMaterial (Variables|Default|GetSphere) 0 "/Game/Level1/Materials/Basic_Green.Basic_Green")
      (Rendering|Material|SetMaterial (Variables|Default|GetStaticMesh) 0 "/Game/Level1/Materials/Basic_Green.Basic_Green")
      (bind _returnvalue (UserInterface|CreateWidget "/Game/Level1/Win_Screen.Win_Screen_C"))
      (UserInterface|Viewport|AddtoViewport _returnvalue 0))))

(fn ConstructionScript)