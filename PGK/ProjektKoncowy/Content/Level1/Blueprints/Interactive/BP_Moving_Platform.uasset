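; BP_Moving_Platform is an interactive platform that moves only while at least two buttons are pressed.
; ButtonActivate and ButtonDeactivate maintain a pressed count, playing the timeline when it reaches two and reversing it when it drops below.
; The timeline's Movement output is added to the world location cached at BeginPlay to position the Platform component, without sweeping.
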(event EventButtonActivate
  (bind _output_get (Variables|Default|SetButtons_Pressed (+ 1 (Variables|Default|GetButtons_Pressed))))
  (if (>= _output_get 2)
    (bind _movement (Timeline|Timeline_0 Play)
      (:Update
        (Transformation|SetWorldLocation (Variables|Default|GetPlatform) (+ _movement (Variables|Default|GetInitial_Location)) false false)))))

(event EventBeginPlay
  (Variables|Default|SetInitial_Location (Transformation|GetWorldLocation (Variables|Default|GetPlatform))))

(event EventButtonDeactivate
  (bind _output_get (Variables|Default|SetButtons_Pressed (- (Variables|Default|GetButtons_Pressed) 1)))
  (if (< _output_get 2)
    (bind _movement (Timeline|Timeline_0 Reverse)
      (:Update
        (Transformation|SetWorldLocation (Variables|Default|GetPlatform) (+ _movement (Variables|Default|GetInitial_Location)) false false)))))

(fn ConstructionScript
  (|CallParentFunction))