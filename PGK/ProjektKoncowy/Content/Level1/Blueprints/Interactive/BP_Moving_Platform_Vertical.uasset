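; Vertical moving platform for Level 1 that responds to button activate and deactivate events.
; It caches the Platform component's world location on BeginPlay, and a timeline adds its Movement offset to that location on each update, without sweep.
; Activation plays the timeline from its current position, while deactivation reverses it from the end, so an interrupted rise jumps to the end offset before returning.
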(event EventButtonActivate
  (if true
    (bind _movement (Timeline|Timeline_0 Play)
      (:Update
        (Transformation|SetWorldLocation (Variables|Default|GetPlatform) (+ _movement (Variables|Default|GetInitial_Location)) false false)))))

(event EventBeginPlay
  (Variables|Default|SetInitial_Location (Transformation|GetWorldLocation (Variables|Default|GetPlatform))))

(event EventButtonDeactivate
  (if true
    (bind _movement (Timeline|Timeline_0 ReverseFromEnd)
      (:Update
        (Transformation|SetWorldLocation (Variables|Default|GetPlatform) (+ _movement (Variables|Default|GetInitial_Location)) false false)))))

(fn ConstructionScript
  (|CallParentFunction))